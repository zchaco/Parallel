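; Player controller for a card game, owning the local player's deck, hand, health and game board UI.
; On BeginPlay it constructs deck and hand objects, sets health to max and creates the board widget, filling it with deck count and life points, with opponent values zeroed as placeholders.
; Pressing F moves a card from deck to hand and prints each hand card's name, without refreshing the UI.
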(event EventBeginPlay
  (CallFunction|CreatDeckObject)
  (CallFunction|CreateHandObject)
  (Variables|Default|SetCurrentHealth (Variables|Default|GetMaxHealth))
  (CallFunction|CreatePlayerUI))

(event EventTick
  (params (DeltaSeconds :type Float%20%28single-precision%29)))

(event Input|KeyboardEvents|F
  (params (Key :type Key%20Structure :default "None"))
  (:Pressed
    (CallFunction|DrawCard)
    (for _array_element (Variables|/Game/Parallel/Core/BP_HandObject.BP_HandObject_C|GetCards (Variables|Default|GetHand))
      (Development|PrintString (Utilities|String|ToString(Name) (Variables|/Game/Parallel/Core/BP_CardObject.BP_CardObject_C|GetName _array_element))))))

(fn ConstructionScript)

(fn DrawCard
  (bind _card (Default|PopCard (Variables|Default|GetDeck)))
  (Default|AddCard (Variables|Default|GetHand) _card))

(fn UpdateGameBoardUI
  (bind _gameboardui (Variables|Default|GetGameBoardUI))
  (Default|UpdateCardsinDeck _gameboardui (Variables|/Game/Parallel/Core/BP_DeckObject.BP_DeckObject_C|GetTotalNumOfCards (Variables|Default|GetDeck)))
  (Default|UpdatePlayerLifePoints _gameboardui (Variables|Default|GetCurrentHealth))
  (Default|UpdateOpponentsCardsinDeck _gameboardui)
  (Default|UpdateOpponentLifePoints _gameboardui))

(fn CreatDeckObject
  ;[1 1 1] Create Deck Object
  (bind _returnvalue (Game|ConstructObjectfromClass "/Game/Parallel/Core/BP_DeckObject.BP_DeckObject_C" self))
  (bind _output_get (Variables|Default|SetDeck _returnvalue))
  (Default|InitDeck _output_get 5))

(fn CreateHandObject
  (bind _returnvalue (Game|ConstructObjectfromClass "/Game/Parallel/Core/BP_HandObject.BP_HandObject_C" self))
  (Variables|Default|SetHand _returnvalue))

(fn CreatePlayerUI
  (bind _returnvalue (UserInterface|CreateWidget "/Game/Parallel/Core/WBP_GameBoardWidget.WBP_GameBoardWidget_C" self))
  (bind _output_get (Variables|Default|SetGameBoardUI _returnvalue))
  (UserInterface|Viewport|AddtoViewport _output_get 0)
  (CallFunction|UpdateGameBoardUI))