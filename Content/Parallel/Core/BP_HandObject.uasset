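; BP_HandObject models a hand of cards, holding a Cards array with functions to add and remove entries.
; Removal by card or by index returns the removed card, logging an expected error on failure.
; The by-card Remove call shows no item wired in, while the by-index path validates the index first.
; IsEmpty returns an Empty value that none of these functions update.
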(fn AddCard
  (params (card :type BP%20Card%20Object%20Object%20Reference))
  (Utilities|Array|Add (Variables|Default|GetCards) card))

(fn RemoveCardbyCard
  (params (card :type BP%20Card%20Object%20Object%20Reference))
  (LocalVariables|SetRemovedCard card)
  (bind _returnvalue (Utilities|Array|RemoveItem (Variables|Default|GetCards) 0))
  (if _returnvalue
    (return (LocalVariables|GetRemovedCard))
    (else
      (Class|AutomationBlueprintFunctionLibrary|AddExpectedLogError "Removed Card Null"))))

(fn RemoveCardbyIndex
  (params (Index :type Integer))
  (bind _cards (Variables|Default|GetCards))
  (bind _output_get (LocalVariables|SetRemoveIndex Index))
  (if (Utilities|Array|IsValidIndex _cards _output_get)
    (LocalVariables|SetRemovedCard (Utilities|Array|Get(acopy) _cards (LocalVariables|GetRemoveIndex)))
    (Utilities|Array|RemoveIndex (Variables|Default|GetCards) (LocalVariables|GetRemoveIndex))
    (return (LocalVariables|GetRemovedCard))
    (else
      (Class|AutomationBlueprintFunctionLibrary|AddExpectedLogError "Removed Card Null"))))

(fn IsEmpty
  (return (Variables|Size|GetbEmpty)))