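; BP_DuelLogic is an early scaffold for the rules of a two-player card duel.
; BeginPlay caches the first player controller as P1, while P2 is never assigned here.
; ImportCards calls an empty GenerateCard per line of test.txt, and pawn and card spawn nodes are unwired.
; Turn events are stubs, and IsGameOver, which checks both players' PlayerState health for zero or below, sits only in unconnected logic.
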(event Custom|Generate%20Card
  (params (Card%20Structure :type Card%20Structure%20Structure)))

(event Custom|InitPlayers
  ;[1 1 1] Initalize Players
  (Utilities|FlowControl|Sequence
    (:then_0
      (bind _asbp_player_controller (Utilities|Casting|CastToBP_PlayerController (Game|GetPlayerController 0)))
      (Variables|GameControl|SetP1 _asbp_player_controller))))

(event Custom|Import%20Cards
  ;[1 1 1] Import Cards
  (for _array_element (.SaveTextA (Class|CardImporter|LoadCards "test.txt"))
    (CallFunction|GenerateCard)))

(event EventBeginPlay
  (CallFunction|InitPlayers))

(event Custom|DrawCard
  (if (Utilities|Enum|Equal(Enum) (Variables|GameControl|GetTurn) "1")
    _))

(event Custom|ResolveAction)

(event Custom|NextTurn)

(event Custom|Click_Attack)

(event Game|Damage|EventAnyDamage
  (params (Damage :type Float%20%28single-precision%29) (DamageType :type Damage%20Type%20Object%20Reference) (InstigatedBy :type Controller%20Object%20Reference) (DamageCauser :type Actor%20Object%20Reference)))

(fn ConstructionScript)

(fn IsGameOver
  (bind _currenthealth (CallFunction|GetPlayerHealth (Variables|GameControl|GetP1)))
  (bind _currenthealth_2 (CallFunction|GetPlayerHealth (Variables|GameControl|GetP2)))
  (if (or (<= _currenthealth_2 0) (<= _currenthealth 0))
    (Variables|GameControl|SetbGameOver true)
    (else
      (Variables|GameControl|SetbGameOver false)))
  (return (Variables|GameControl|GetbGameOver)))

(fn GetPlayerHealth
  (params (PlayerController :type Controller%20Object%20Reference))
  (bind _asbp_player_state (Utilities|Casting|CastToBP_PlayerState (Variables|/Script/Engine.Controller|GetPlayerState PlayerController))
    (:then
      _)
    (:CastFailed
      _))
  (return (Variables|/Game/Parallel/Core/BP_PlayerState.BP_PlayerState_C|GetCurrentHealth _asbp_player_state)))